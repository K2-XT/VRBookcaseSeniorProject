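; Overlap volume that cleans up interactable objects entering it, destroying them or sending key platforms back to their level defaults.
; On actor overlap it ignores anything not derived from BP_Interactive_Object, protecting the player and scenery.
; Spawn and level-end platforms are moved to the first default spawn or end location actor found in the level.
; All other interactables are destroyed.
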(event `self.ReceiveActorBeginOverlap`
  (params (OtherActor :type "Actor Object Reference"))
  (`self.DestroyOrTeleportObject` OtherActor))

(fn `DestroyOrTeleportObject`
  (params (Object :type "Object Object Reference"))
  ;[1 1 1] Check if it is an interactable, we don't want to destory any other type of object, otherwise we could be destroying bookcases, the player, the floor...
  (bind _asbp_interactive_object (cast `/Game/Blueprints/InteractableObjects/BP_Interactive_Object` Object))
  ;[1 1 1] If the Interactable is a Spawn Platform, telelport to default spawn in level.
  (bind _asbp_action_figure_spawn (cast `/Game/Blueprints/NextLevelAndActionFigureSpawners/BP_Action_Figure_Spawn` _asbp_interactive_object)
    (:`then`
      (bind _outactors (`GameplayStatics.GetAllActorsOfClass` "/Game/Blueprints/NextLevelAndActionFigureSpawners/BP_Default_Spawn_Location.BP_Default_Spawn_Location_C"))
      (`self.K2_SetActorTransform` _asbp_action_figure_spawn (`self.GetTransform` (`|GetArrayItem` _outactors)) false false))
    (:`CastFailed`
      ;[1 1 1] If the object is an End Platform, teleport back to the default end spawn in level.
      (bind _asbp_level_end (cast `/Game/Blueprints/NextLevelAndActionFigureSpawners/BP_Level_End` _asbp_interactive_object)
        (:`then`
          (bind _outactors_2 (`GameplayStatics.GetAllActorsOfClass` "/Game/Blueprints/NextLevelAndActionFigureSpawners/BP_Default_End_Location.BP_Default_End_Location_C"))
          (`self.K2_SetActorTransform` _asbp_level_end (`self.GetTransform` (`|GetArrayItem` _outactors_2)) false false))
        (:`CastFailed`
          ;[1 1 1] If the object is any other interactable, destory it.
          (`self.K2_DestroyActor` _asbp_interactive_object))))))

(fn `UserConstructionScript`)