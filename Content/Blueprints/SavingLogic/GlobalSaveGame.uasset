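; Global save game that stores each level's interactables data in an ordered Levels array, keyed by level name.
; SaveLevelData overwrites a matching entry or appends a new one, while GetLevelData returns the cached Interactables if no name matches.
; ClearLevelData removes a level, then renames all remaining entries by array index as "Level{int}".
; GetNextLevel uses array order to return the following level's name, or an empty string after the last.
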(fn `ClearIndexOfCurrentLevel`
  (params (levelName :type String))
  (for (_array_element _array_index) (`self.levels`)
    ;[1 1 1] If the given level exists...
    (if (`KismetStringLibrary.EqualEqual_StrStr` levelName (`.LevelName_2_A9B1EF6443079C2B2D931DBBC6E84215` (break `/Game/Blueprints/SavingLogic/LevelSaveData` _array_element)))
      ;[1 1 1] Remove it from the array of levels.
      (`KismetArrayLibrary.Array_Remove` (`self.levels`) _array_index))))

(fn `ClearLevelData`
  (params (levelName :type String))
  (`self.ClearIndexOfCurrentLevel` levelName)
  (`self.ReassignLevelNames`)
  (return))

(fn `GetLevelData`
  (params (levelName :type String))
  (returns (interactablesData :type "Array of /Game/Blueprints/SavingLogic/InteractableSaveData Structure"))
  (for _array_element (`self.levels`)
    (bind (_levelname _interactablesdata) (break `/Game/Blueprints/SavingLogic/LevelSaveData` _array_element))
    ;[1 1 1] If we can find the given level in our levels, return it's held data.
    (if (`KismetStringLibrary.EqualEqual_StrStr` _levelname levelName)
      (bind _output_get (set `self.interactables` _interactablesdata))
      (return _output_get)))
  ;[1 1 1] If the level was not found, return the last loaded level to avoid bad situations.
  (return (`self.interactables`)))

(fn `GetNextLevel`
  (params (levelName :type String))
  (returns (nextLevelName :type String))
  (locals (nextIndex :type Integer))
  (bind _levels (`self.levels`))
  (for (_array_element _array_index) (`self.levels`)
    ;[1 1 1] Find the current level, then get it's index++ to find the next level.
    (if (`KismetStringLibrary.EqualEqual_StrStr` (`.LevelName_2_A9B1EF6443079C2B2D931DBBC6E84215` (break `/Game/Blueprints/SavingLogic/LevelSaveData` _array_element)) levelName)
      (bind _result (`/Engine/EditorBlueprintResources/StandardMacros.IncrementInt` _array_index)
        (:`  `
          (bind _output_get (set `local.nextIndex` _result))
          ;[1 1 1] However, there may not be a next level to load. We may be at the end of our levels.
          (if (`KismetArrayLibrary.Array_IsValidIndex` _levels _output_get)
            ;[1 1 1] If we're at the end of our levels, return an empty level name. Otherwise, return the next level's name.
            (return (`.LevelName_2_A9B1EF6443079C2B2D931DBBC6E84215` (break `/Game/Blueprints/SavingLogic/LevelSaveData` (`|GetArrayItem` _levels (`local.nextIndex`)))))
            (else
              (return ""))))))))

(fn `ReassignLevelNames`
  (for (_array_element _array_index) (`self.levels`)
    ;[1 1 1] Then re-assign each level's name to the generated name.
    (`KismetArrayLibrary.Array_Set` (`self.levels`) _array_index (make `/Game/Blueprints/SavingLogic/LevelSaveData` (`KismetTextLibrary.Conv_TextToString` (`|FormatText` "Level{int}" _array_index)) (`.InteractablesData_6_30EB2BF347908E0719CC19A23C9DA740` (break `/Game/Blueprints/SavingLogic/LevelSaveData` _array_element))) true)))

(fn `SaveLevelData`
  (params (LevelName :type String) (Interactables :type "Array of /Game/Blueprints/SavingLogic/InteractableSaveData Structure"))
  (bind _levelsavedata (make `/Game/Blueprints/SavingLogic/LevelSaveData` LevelName (`self.interactables`)))
  ;[1 1 1] First, set our interactables data to the data of the data we are given. (Expected: The level being worked on.
  (set `self.interactables` Interactables)
  (for (_array_element _array_index) (`self.levels`)
    ;[1 1 1] If the level exists, override the existing data with the new data and return.
    (if (`KismetStringLibrary.EqualEqual_StrStr` (`.LevelName_2_A9B1EF6443079C2B2D931DBBC6E84215` (break `/Game/Blueprints/SavingLogic/LevelSaveData` _array_element)) LevelName)
      (`KismetArrayLibrary.Array_Set` (`self.levels`) _array_index _levelsavedata)
      (return)))
  ;[1 1 1] If we get through all the levels without finding the given level, it must be a new level, and should be added.
  (`KismetArrayLibrary.Array_Add` (`self.levels`) _levelsavedata)
  (return))