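; RootGameInstance is a game instance Blueprint that sets up the game's persistent save data at startup.
; On Init it checks for a save in the configured slot and, if one exists, loads it, casts it to GlobalSaveGame and caches it in SaveGameData.
; Otherwise it creates a new GlobalSaveGame, caches it the same way and immediately writes it to the slot.
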(event `self.ReceiveInit`
  ;[1 1 1] Have we already created a save game in the past?
  (bind _returnvalue (`GameplayStatics.DoesSaveGameExist` (`self.saveSlotName`)))
  (if _returnvalue
    ;[1 1 1] If we have, load it up and store it in a variable.
    (bind _returnvalue_2 (`GameplayStatics.LoadGameFromSlot` (`self.saveSlotName`)))
    (bind _asglobal_save_game (cast `/Game/Blueprints/SavingLogic/GlobalSaveGame` _returnvalue_2))
    (set `self.saveGameData` _asglobal_save_game)
    (else
      ;[1 1 1] If we don't already have a save game, create a new save game object and save it to our slot.
      (bind _returnvalue_3 (`GameplayStatics.CreateSaveGameObject` "/Game/Blueprints/SavingLogic/GlobalSaveGame.GlobalSaveGame_C"))
      (bind _output_get (set `self.saveGameData` _returnvalue_3))
      (`GameplayStatics.SaveGameToSlot` _output_get (`self.saveSlotName`)))))