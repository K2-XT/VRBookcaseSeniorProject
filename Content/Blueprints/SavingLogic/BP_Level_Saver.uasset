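; BP_Level_Saver is a grabbable object that saves the current level's interactables when grabbed.
; It gathers every BP_Interactive_Object flagged for saving into structs holding type ID, box transform and frozen state.
; SaveObjects stores that array under the level name in the game instance's shared save data and writes it to the save slot.
; It then reads the data back to print a count for development feedback.
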(fn `Fill Temp Interactables`
  (params (tempInteractables :type "Array of /Game/Blueprints/SavingLogic/InteractableSaveData Structure (by ref)"))
  (bind _outactors (`GameplayStatics.GetAllActorsOfClass` "/Game/Blueprints/InteractableObjects/BP_Interactive_Object.BP_Interactive_Object_C"))
  (for _array_element _outactors
    ;[1 1 1] Check the object if we save it. If we don't need to, don't worry about it.
    (if (`/Game/Blueprints/InteractableObjects/BP_Interactive_Object.doWeSaveObject` _array_element)
      ;[1 1 1] Get the relevant data needed to spawn the object upon a level load, save it into a struct, and add it to the array we were given.
      (`KismetArrayLibrary.Array_Add` tempInteractables (make `/Game/Blueprints/SavingLogic/InteractableSaveData` (`/Game/Blueprints/InteractableObjects/BP_Interactive_Object.InteractableID` _array_element) (`SceneComponent.K2_GetComponentToWorld` (`/Game/Blueprints/InteractableObjects/BP_Interactive_Object.Box` _array_element)) (`/Game/Blueprints/InteractableObjects/BP_Interactive_Object.isFrozen` _array_element)))))
  (return))

(fn `Grab`
  (params (parent :type "SceneComponent Object Reference"))
  ;[1 1 1] In this object, we just want to save the current level when grabbed.
  (`self.SaveObjects` (`/Game/Blueprints/SavingLogic/RootGameInstance.currentLevel` (`self.currentGameInstance`))))

(fn `SaveObjects`
  (params (currentLevelName :type String))
  (locals (tempInteractables :type "Array of /Game/Blueprints/SavingLogic/InteractableSaveData Structure"))
  (bind _currentgameinstance (`self.currentGameInstance`))
  (bind _savegamedata (`/Game/Blueprints/SavingLogic/RootGameInstance.saveGameData` _currentgameinstance))
  ;[1 1 1] Fill local variable tempInteractables with all the interactables we're supposed to save in the current level. Then save that into our singleton save game data.
  (`self.Fill Temp Interactables` (`local.tempInteractables`))
  (`/Game/Blueprints/SavingLogic/GlobalSaveGame.SaveLevelData` (`/Game/Blueprints/SavingLogic/RootGameInstance.saveGameData` (`self.currentGameInstance`)) currentLevelName (`local.tempInteractables`))
  ;[1 1 1] Save our singleton save data into a slot within the game instance.
  (`GameplayStatics.SaveGameToSlot` _savegamedata (`/Game/Blueprints/SavingLogic/RootGameInstance.saveSlotName` _currentgameinstance))
  ;[1 1 1] Pull the data we just saved back out for verification in development.
  (bind _interactablesdata (`/Game/Blueprints/SavingLogic/GlobalSaveGame.GetLevelData` _savegamedata (`local.CurrentLevelName`)))
  ;[1 1 1] Let's the developer know that SOMETHING was saved. Not a for sure garauntee until the level is reloaded.
  (`KismetSystemLibrary.PrintString` (`KismetTextLibrary.Conv_TextToString` (`|FormatText` "Was able to save {int} interactables into level: {string}" (`KismetStringLibrary.Conv_IntToString` (`KismetArrayLibrary.Array_Length` _interactablesdata)) (`local.CurrentLevelName`))) true true (struct :`R` 0.321725 :`G` 1.0 :`A` 1.0) 5.0))

(fn `UserConstructionScript`
  (`parent.UserConstructionScript`))