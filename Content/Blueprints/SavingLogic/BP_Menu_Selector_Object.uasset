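; BP_Menu_Selector_Object is an interactive object base for menu buttons, many of whose children act as save buttons.
; It highlights on actor overlap and routes Interact to Grab or Drop, both empty here.
; BeginPlay caches the RootGameInstance for children and excludes the object from saving.
; Activate and the kinetic rotate, pull and push events are deliberately stubbed out to suppress normal BP_Interactive_Object behavior.
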(event `self.ReceiveActorBeginOverlap`
  (params (OtherActor :type "Actor Object Reference"))
  ;[1 1 1] These are the actual i_interactables functions that needed handling.
  (`self.HandleObjectOverlapHighlighting` OtherActor))

(event `self.ReceiveActorEndOverlap`
  (params (OtherActor :type "Actor Object Reference"))
  ;[1 1 1] These are the actual i_interactables functions that needed handling.
  (`self.HandleObjectOverlapUnhighlighting` OtherActor))

(event `/Game/Blueprints/iInteractable.Interact`
  (params (Hand :type "SceneComponent Object Reference") (bHolding :type Boolean))
  ;[1 1 1] These are the actual i_interactables functions that needed handling.
  (if bHolding
    (`self.Grab` null)
    (else
      (`self.Drop`))))

(event `self.ReceiveBeginPlay`
  (`parent.ReceiveBeginPlay`)
  ;[1 1 1] Because a good amount of children will be saving buttons visible to the player, we're going to need to access the game instance. So here I save it into a variable the children can access.
  (bind _asroot_game_instance (cast `/Game/Blueprints/SavingLogic/RootGameInstance` (`GameplayStatics.GetGameInstance`)))
  (set `self.currentGameInstance` _asroot_game_instance)
  ;[1 1 1] We never want our game to save our menu buttons.
  (set `self.doWeSaveObject` false))

(event `/Game/Blueprints/iInteractable.Activate`
  ;[1 1 1] I didn't want anything to happen when the player tried to do these normal BP_Interactive_Object implementations, so I just tied these i_interactables calls to nothing.
)

(event `/Game/Blueprints/iInteractable.RotateObjectKinetically`
  (params (isRotatingLeft :type Boolean) (CollisionBox :type "PrimitiveComponent Object Reference"))
  ;[1 1 1] I didn't want anything to happen when the player tried to do these normal BP_Interactive_Object implementations, so I just tied these i_interactables calls to nothing.
)

(event `/Game/Blueprints/iInteractable.PullObjectKinetically`
  (params (Hand :type "SceneComponent Object Reference") (CollisionBox :type "PrimitiveComponent Object Reference"))
  ;[1 1 1] I didn't want anything to happen when the player tried to do these normal BP_Interactive_Object implementations, so I just tied these i_interactables calls to nothing.
)

(event `/Game/Blueprints/iInteractable.PushObjectKinetically`
  (params (Hand :type "SceneComponent Object Reference") (CollisionBox :type "PrimitiveComponent Object Reference"))
  ;[1 1 1] I didn't want anything to happen when the player tried to do these normal BP_Interactive_Object implementations, so I just tied these i_interactables calls to nothing.
)

(fn `Drop`)

(fn `Grab`
  (params (parent :type "SceneComponent Object Reference")))

(fn `UserConstructionScript`
  (`parent.UserConstructionScript`))