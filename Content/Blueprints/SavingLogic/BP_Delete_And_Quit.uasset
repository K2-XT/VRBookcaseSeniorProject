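; BP_Delete_And_Quit is a grabbable actor that deletes the current level's saved data and returns the player to the main menu.
; Its Grab function clears the current level's object data from the game instance's SaveGameData, then writes the save to its slot.
; It then opens MainMenu, signalling the deletion and avoiding cleanup of objects left in the open level.
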(fn `Grab`
  (params (parent :type "SceneComponent Object Reference"))
  (bind _currentgameinstance (`self.currentGameInstance`))
  (bind _savegamedata (`/Game/Blueprints/SavingLogic/RootGameInstance.saveGameData` _currentgameinstance))
  ;[1 1 1] Destroy the array of object data that represents the current level from the saveGameData.
  (`/Game/Blueprints/SavingLogic/GlobalSaveGame.ClearLevelData` _savegamedata (`/Game/Blueprints/SavingLogic/RootGameInstance.currentLevel` _currentgameinstance))
  (`GameplayStatics.SaveGameToSlot` _savegamedata (`/Game/Blueprints/SavingLogic/RootGameInstance.saveSlotName` _currentgameinstance))
  ;[1 1 1] Then exit to the main menu to communicate to the user that the level has been destroyed and allow them to create new ones if wanted. Also saves us a headache of how we would handle the leftover objects if we kept the user in the currently worked on level.
  (`GameplayStatics.OpenLevelBySoftObjectPtr` "/Game/Maps/MainMenu.MainMenu"))

(fn `UserConstructionScript`
  (`parent.UserConstructionScript`))