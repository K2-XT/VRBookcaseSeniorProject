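; Level editor bookcase that presents five wooden block types: cube, ramp, cylinder, long and rectangle.
; It is a child Blueprint that sets its bookcase name to "WoodenBlocks" in the construction script.
; On BeginPlay it passes the block classes to the parent's fill function, then calls SpawnObjectsAndSpawners to create the objects and their spawners.
; An older manual array-filling chain remains in the graph but never runs.
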(event `self.ReceiveBeginPlay`
  (`parent.ReceiveBeginPlay`)
  (`self.FillArrayOfObjectsToPresent` "/Game/Blueprints/InteractableObjects/WoodenBlocks/BP_Wooden_Cube.BP_Wooden_Cube_C" "/Game/Blueprints/InteractableObjects/WoodenBlocks/BP_WoodenRamp.BP_WoodenRamp_C" "/Game/Blueprints/InteractableObjects/WoodenBlocks/BP_Wooden_Cylinder.BP_Wooden_Cylinder_C" "/Game/Blueprints/InteractableObjects/WoodenBlocks/BP_Wooden_Long.BP_Wooden_Long_C" "/Game/Blueprints/InteractableObjects/WoodenBlocks/BP_Wooden_Rectangle.BP_Wooden_Rectangle_C")
  (`self.SpawnObjectsAndSpawners`))

(fn `UserConstructionScript`
  (set `self.bookcaseName` "WoodenBlocks")
  (`parent.UserConstructionScript`))