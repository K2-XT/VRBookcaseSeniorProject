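; Base level editor bookcase that displays a named set of interactable objects on up to six spawn points.
; Its construction script gathers the spawn point components and labels the top shelf with the bookcase name.
; A fill function stores the objects, and a spawn function creates an interactable spawner for each at the matching point.
; Deconstruction stops and destroys every interactable spawner in the level and their overlapping interactive objects, then the bookcase.
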(fn `DeconstructBookcase`
  (bind _outactors (`GameplayStatics.GetAllActorsOfClass` "/Game/Blueprints/LevelEditorBookcases/BP_Interactable_Spawner.BP_Interactable_Spawner_C"))
  (for _array_element _outactors
    ;[1 1 1] For each interactable spawner, tell it to stop spawning. Then find all the overlapping interactables and destroy them.
    (bind _asbp_interactable_spawner (cast `/Game/Blueprints/LevelEditorBookcases/BP_Interactable_Spawner` _array_element))
    (set `/Game/Blueprints/LevelEditorBookcases/BP_Interactable_Spawner.stopSpawning` true _asbp_interactable_spawner)
    (for _array_element_2 (`self.GetOverlappingActors` _array_element "/Game/Blueprints/InteractableObjects/BP_Interactive_Object.BP_Interactive_Object_C")
      (`self.K2_DestroyActor` _array_element_2))
    (`self.K2_DestroyActor` _array_element))
  ;[1 1 1] Then destroy the bookcase.
  (`self.K2_DestroyActor`))

(fn `FillArrayOfObjectsToPresent`
  (params (object :type "/Game/Blueprints/InteractableObjects/BP_Interactive_Object Class Reference") (object1 :type "/Game/Blueprints/InteractableObjects/BP_Interactive_Object Class Reference") (object2 :type "/Game/Blueprints/InteractableObjects/BP_Interactive_Object Class Reference") (object3 :type "/Game/Blueprints/InteractableObjects/BP_Interactive_Object Class Reference") (object4 :type "/Game/Blueprints/InteractableObjects/BP_Interactive_Object Class Reference") (object5 :type "/Game/Blueprints/InteractableObjects/BP_Interactive_Object Class Reference"))
  (set `self.arrayOfObjectsToPresent` (`|MakeArray` object object1 object2 object3 object4 object5 :!type "Actor Class Reference")))

(fn `SpawnObjectsAndSpawners`
  (for (_array_element _array_index) (`self.arrayOfObjectsToPresent`)
    ;[1 1 1] Get the array of spawn locations, and spawn an interactable spawner.
    (bind _returnvalue (`|SpawnActorFromClass` "/Game/Blueprints/LevelEditorBookcases/BP_Interactable_Spawner.BP_Interactable_Spawner_C" (`SceneComponent.K2_GetComponentToWorld` (`|GetArrayItem` (`self.arrayOfSpawnPoints`) _array_index)) "AlwaysSpawn" "OverrideRootScale" null null))
    (if true
      ;[1 1 1] Set the object to spawn it the spawner and set it.
      (set `/Game/Blueprints/LevelEditorBookcases/BP_Interactable_Spawner.objectToSpawn` _array_element _returnvalue)
      (`/Game/Blueprints/LevelEditorBookcases/BP_Interactable_Spawner.SpawnObject` _returnvalue))))

(fn `UserConstructionScript`
  ;[1 1 1] Fill Array of Spawners
  (set `self.arrayOfSpawnPoints` (`|MakeArray` (`self.SC_BookcaseObjectSpawner`) (`self.SC_BookcaseObjectSpawner1`) (`self.SC_BookcaseObjectSpawner2`) (`self.SC_BookcaseObjectSpawner3`) (`self.SC_BookcaseObjectSpawner4`) (`self.SC_BookcaseObjectSpawner5`) :!type "SceneComponent Object Reference"))
  ;[1 1 1] Set the top shelf text to the name of the objects to display.
  (`TextRenderComponent.K2_SetText` (`self.TextRender`) (`self.bookcaseName`)))