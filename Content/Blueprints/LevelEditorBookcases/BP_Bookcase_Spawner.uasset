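; BP_Bookcase_Spawner is a level editor actor that requests the spawning of a chosen bookcase.
; SpawnBookcaseAtSpawner finds all BP_Bookcase_Spawn_Point actors and passes the bookcase to the first one's SpawnBookcase, so it effectively relies on a single spawn point.
; Its Grab override only calls the parent, and its event graph holds no active logic.
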(fn `Grab`
  (params (parent :type "SceneComponent Object Reference"))
  (`parent.Grab` null))

(fn `SpawnBookcaseAtSpawner`
  (params (BookcaseToSpawn :type "/Game/Blueprints/LevelEditorBookcases/BP_EditorBookcaseBase Class Reference"))
  (bind _outactors (`GameplayStatics.GetAllActorsOfClass` "/Game/Blueprints/LevelEditorBookcases/BP_Bookcase_Spawn_Point.BP_Bookcase_Spawn_Point_C"))
  (`/Game/Blueprints/LevelEditorBookcases/BP_Bookcase_Spawn_Point.SpawnBookcase` (`|GetArrayItem` _outactors) BookcaseToSpawn))

(fn `UserConstructionScript`
  (`parent.UserConstructionScript`))