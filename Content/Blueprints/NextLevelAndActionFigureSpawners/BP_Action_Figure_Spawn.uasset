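; Spawner actor that places a VR_ActionFigure at the transform of its SCSpawnActionFigure component.
; Both the construction script and BeginPlay call the spawn function, though the author's comment reports only one spawn occurring, cause untested.
; The construction script also sets the spawner's interactable ID, frozen state and save flag.
; BeginPlay re-freezes the spawner under VRSideScrollerGameMode, to prevent player modification outside the editor.
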(event `self.ReceiveBeginPlay`
  (`parent.ReceiveBeginPlay`)
  ;[1 1 1] Spawn the action figure. If we're not in the editor, we do not want the player to be able to modify this object. So freeze it.
  (`self.SpawnActionFigure`)
  (cast `/Game/Blueprints/GameModes/VRSideScrollerGameMode` (`GameplayStatics.GetGameMode`))
  (set `self.isFrozen` true))

(fn `SpawnActionFigure`
  (`|SpawnActorFromClass` "/Game/Blueprints/VR_ActionFigure.VR_ActionFigure_C" (`SceneComponent.K2_GetComponentToWorld` (`self.SC_Spawn_Action_Figure`)) "AdjustIfPossibleButAlwaysSpawn" "OverrideRootScale" null null))

(fn `UserConstructionScript`
  (`parent.UserConstructionScript`)
  ;[1 1 1] So, I implemented this both here and on BeginPlay, but it only runs once despite it being both here and there. Futher testing is required to see which one is actually executing.
  (set `self.InteractableID` "NewEnumerator6")
  (set `self.isFrozen` true)
  (set `self.doWeSaveObject` true)
  (`self.SpawnActionFigure`))