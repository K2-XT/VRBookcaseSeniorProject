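; BP_Level_End is a saveable, frozen level-end interactable that advances the player to the next level when the action figure reaches it.
; On BeginPlay it asks the game instance's save data for the level after the current one.
; On overlap, only in the VR side-scroller game mode, it destroys the action figure, then sets that level as current and opens DefaultLevel, or opens MainMenu when none remains.
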(event `self.ReceiveBeginPlay`
  (`parent.ReceiveBeginPlay`)
  ;[1 1 1] We always want to save this object, and we always want it to start frozen.
  (set `self.isFrozen` true)
  (set `self.doWeSaveObject` true)
  ;[1 1 1] Access the current game instance and get the current level. Then find the next level and set our member variable to the next level.
  (bind _asroot_game_instance (cast `/Game/Blueprints/SavingLogic/RootGameInstance` (`GameplayStatics.GetGameInstance`)))
  (bind _output_get (set `self.currentGameInstance` _asroot_game_instance))
  (bind _nextlevelname (`/Game/Blueprints/SavingLogic/GlobalSaveGame.GetNextLevel` (`/Game/Blueprints/SavingLogic/RootGameInstance.saveGameData` (`self.currentGameInstance`)) (`/Game/Blueprints/SavingLogic/RootGameInstance.currentLevel` _output_get)))
  (set `self.nextLevel` _nextlevelname))

(event `self.ReceiveActorBeginOverlap`
  (params (OtherActor :type "Actor Object Reference"))
  (`parent.ReceiveActorBeginOverlap` OtherActor)
  ;[1 1 1] When the action figure lands, destroy it. It will respawn upon the next level loading. We only want this to happen in the side-scroller gamemode, as it would be inconvenient to the player to destroy their level and load the next if the action figure hit the level end on accident.
  (cast `/Game/Blueprints/GameModes/VRSideScrollerGameMode` (`GameplayStatics.GetGameMode`))
  (bind _asvr_action_figure (cast `/Game/Blueprints/VR_ActionFigure` OtherActor))
  (`self.K2_DestroyActor` _asvr_action_figure)
  ;[1 1 1] If the nextLevel string is empty, that means we're out of levels. Return to the main menu. If not, open the next level.
  (if (`KismetStringLibrary.EqualEqual_StrStr` "" (`self.nextLevel`))
    (`GameplayStatics.OpenLevelBySoftObjectPtr` "/Game/Maps/MainMenu.MainMenu")
    (else
      (set `/Game/Blueprints/SavingLogic/RootGameInstance.currentLevel` (`self.nextLevel`) (`self.currentGameInstance`))
      (`GameplayStatics.OpenLevelBySoftObjectPtr` "/Game/Maps/DefaultLevel.DefaultLevel"))))

(fn `UserConstructionScript`
  (`parent.UserConstructionScript`)
  (set `self.InteractableID` "NewEnumerator7")
  (set `self.isFrozen` true)
  (set `self.doWeSaveObject` true))