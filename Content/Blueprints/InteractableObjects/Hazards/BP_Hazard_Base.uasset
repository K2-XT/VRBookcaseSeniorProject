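; BP_Hazard_Base is a hazard actor, named as a base, that destroys any VR action figure overlapping it and triggers a replacement.
; On overlap it casts the other actor to VR_ActionFigure and ignores anything else.
; After destroying the figure, it looks up the level's BP_Action_Figure_Spawn actors and calls SpawnActionFigure on the first one found.
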(event `self.ReceiveActorBeginOverlap`
  (params (OtherActor :type "Actor Object Reference"))
  (`parent.ReceiveActorBeginOverlap` OtherActor)
  ;[1 1 1] If the overlapping object is an action figure, destroy it and tell the spawner in the level to spawn a new one.
  (bind _asvr_action_figure (cast `/Game/Blueprints/VR_ActionFigure` OtherActor))
  (`self.K2_DestroyActor` _asvr_action_figure)
  (bind _outactors (`GameplayStatics.GetAllActorsOfClass` "/Game/Blueprints/NextLevelAndActionFigureSpawners/BP_Action_Figure_Spawn.BP_Action_Figure_Spawn_C"))
  (`/Game/Blueprints/NextLevelAndActionFigureSpawners/BP_Action_Figure_Spawn.SpawnActionFigure` (`|GetArrayItem` _outactors)))

(fn `UserConstructionScript`
  (`parent.UserConstructionScript`))