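; Base VR interactable object that can be grabbed, pushed, pulled, rotated, and highlighted via custom depth when the VRPawn overlaps it.
; Grabbing disables physics and attaches to the hand, while push, pull and rotate move the Box in small steps and carry the collision box along.
; In VREditorGameMode, Activate toggles a mid-air freeze that saves velocity; outside it, frozen objects cannot be grabbed.
; Overlapping a bookcase spawner marks the object not to be saved.
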(event `self.ReceiveActorBeginOverlap`
  (params (OtherActor :type "Actor Object Reference"))
  (`self.HandleObjectOverlapHighlighting` OtherActor)
  ;[1 1 1] If we are overlapping an object spawner on the bookcase, don't save the object. This is so that we don't have floating objects where the bookcase would be in the play level.
  (cast `/Game/Blueprints/LevelEditorBookcases/BP_Interactable_Spawner` OtherActor)
  (set `self.doWeSaveObject` false))

(event `/Game/Blueprints/iInteractable.PullObjectKinetically`
  (params (Hand :type "SceneComponent Object Reference") (CollisionBox :type "PrimitiveComponent Object Reference"))
  (`self.HandleObjectPulling` CollisionBox Hand))

(event `self.ReceiveActorEndOverlap`
  (params (OtherActor :type "Actor Object Reference"))
  (`self.HandleObjectOverlapUnhighlighting` OtherActor)
  ;[1 1 1] If the object is not overlapping a spawner, it's okay to save.
  (cast `/Game/Blueprints/LevelEditorBookcases/BP_Interactable_Spawner` OtherActor)
  (set `self.doWeSaveObject` true))

(event `/Game/Blueprints/iInteractable.Activate`
  ;[1 1 1] If we are editing, allow freezing/unfreezing.
  (cast `/Game/Blueprints/GameModes/VREditorGameMode` (`GameplayStatics.GetGameMode`))
  (if (`self.isFrozen`)
    (`self.UnfreezeObject`)
    (else
      (`self.FreezeObject`))))

(event `/Game/Blueprints/iInteractable.PushObjectKinetically`
  (params (Hand :type "SceneComponent Object Reference") (CollisionBox :type "PrimitiveComponent Object Reference"))
  (`self.HanldeObjectPushing` CollisionBox Hand))

(event `/Game/Blueprints/iInteractable.RotateObjectKinetically`
  (params (isRotatingLeft :type Boolean) (CollisionBox :type "PrimitiveComponent Object Reference"))
  (`self.HandleObjectRotating` isRotatingLeft CollisionBox))

(event `/Game/Blueprints/iInteractable.Interact`
  (params (Hand :type "SceneComponent Object Reference") (bHolding :type Boolean))
  ;[1 1 1] If we are in the editor, always allow grabbing. If not, conditional grabbing.
  (cast `/Game/Blueprints/GameModes/VREditorGameMode` (`GameplayStatics.GetGameMode`)
    (:`then`
      (`self.HandleEditorGrabbing` bHolding Hand))
    (:`CastFailed`
      (`self.HandleNonEditorGrabbing` bHolding Hand))))

(fn `Drop`
  (bind _box (`self.Box`))
  ;[1 1 1] Detach from the holding component, then check if we detached because we ewere frozen or because we were dropped.
  (`self.K2_DetachFromActor` "KeepWorld" "KeepWorld" "KeepWorld")
  (if (not (`self.isFrozen`))
    ;[1 1 1] If we were just dropped, re-enable physics and gravity.
    (`PrimitiveComponent.SetSimulatePhysics` _box true)
    (`PrimitiveComponent.SetEnableGravity` _box true))
  ;[1 1 1] Either way, our object is no longer being held.
  (set `self.isHeld` false))

(fn `FreezeObject`
  (bind _box (`self.Box`))
  ;[1 1 1] Detach from controller that is holding the object.
  (if (`self.isHeld`)
    (`self.K2_DetachFromActor` "KeepWorld" "KeepWorld" "KeepWorld")
    (set `self.isHeld` false))
  ;[1 1 1] Save velocity for later.
  (set `self.savedVelocity` (`SceneComponent.GetComponentVelocity` _box))
  ;[1 1 1] Stop physics from simulating, zero-out velocity, and disable gravity... effectively "freezing" object in mid-air.
  (`PrimitiveComponent.SetSimulatePhysics` _box false)
  (`PrimitiveComponent.SetPhysicsLinearVelocity` _box (0.0 0.0 0.0) false "None")
  (`PrimitiveComponent.SetEnableGravity` _box false)
  (`PrimitiveComponent.SetPhysicsAngularVelocityInRadians` _box (0.0 0.0 0.0) false "None")
  ;[1 1 1] Indicate we are now frozen.
  (set `self.isFrozen` true))

(fn `Grab`
  (params (parent :type "SceneComponent Object Reference"))
  ;[1 1 1] Stop simulating physics and attach to controller. Yes, this means that the object will no longer collide with most objects, but it's a tradeoff that I have yet to find a way around.
  (`PrimitiveComponent.SetSimulatePhysics` (`self.Box`) false)
  (`self.K2_AttachToComponent` parent "None" "KeepWorld" "KeepWorld" "KeepWorld" false)
  ;[1 1 1] Set our state variables.
  (set `self.isHeld` true)
  (set `self.isFrozen` false))

(fn `HandleEditorGrabbing`
  (params (condition :type Boolean) (parent :type "SceneComponent Object Reference"))
  (if condition
    (`self.Grab` parent)
    (else
      (`self.Drop`))))

(fn `HandleNonEditorGrabbing`
  (params (condition :type Boolean) (parent :type "SceneComponent Object Reference"))
  ;[1 1 1] If we are not in the editor, we do not want to allow the player to unfreeze or manipulate frozen objects.
  (if (`self.isFrozen`)
    _
    (elif condition
      (`self.Grab` parent)
      (else
        (`self.Drop`)))))

(fn `HandleObjectOverlapHighlighting`
  (params (otherActor :type "Actor Object Reference"))
  (bind _box (`self.Box`))
  ;[1 1 1] Check to see what is overlapping us.
  (cast `/Game/Blueprints/VRPawn` otherActor
    (:`then`
      ;[1 1 1] If it's the VRPawn, highlight and break from the loop so we don't accidentally uncheck it later if multiple actors are overlapping.
      (`PrimitiveComponent.SetRenderCustomDepth` _box true))
    (:`CastFailed`
      ;[1 1 1] If it's something else, do nothing.
      (`PrimitiveComponent.SetRenderCustomDepth` _box false))))

(fn `HandleObjectOverlapUnhighlighting`
  (params (object :type "Object Object Reference"))
  ;[1 1 1] If the object that has un-overlapped is the pawn, unhighlight.
  (cast `/Game/Blueprints/VRPawn` object)
  (`PrimitiveComponent.SetRenderCustomDepth` (`self.Box`) false))

(fn `HandleObjectPulling`
  (params (collisionBox :type "PrimitiveComponent Object Reference") (hand :type "SceneComponent Object Reference"))
  (bind _returnvalue (`SceneComponent.K2_GetComponentLocation` hand))
  (bind _box (`self.Box`))
  ;[1 1 1] Set the location of both our object and the collision box that is overlapping it to the new location we calculated. We need to set the collision box's location as well, or else the object will move outside the collision box and we'll be stuck with a floating object attached to the controller.
  (`SceneComponent.K2_SetWorldLocation` _box (+ (* (`SceneComponent.GetForwardVector` hand) (- (`KismetMathLibrary.Vector_Distance` (`SceneComponent.K2_GetComponentLocation` (`self.Box`)) _returnvalue) 2.0)) _returnvalue) true false)
  (`SceneComponent.K2_SetWorldLocation` collisionBox (`SceneComponent.K2_GetComponentLocation` _box) true false))

(fn `HandleObjectRotating`
  (params (condition :type Boolean) (collisionBox :type "PrimitiveComponent Object Reference"))
  ;[1 1 1] Set the collision box to the same location of the object so that the object does not slip out of the collision box while rotating.
  (`SceneComponent.K2_SetWorldLocation` collisionBox (`SceneComponent.K2_GetComponentLocation` (`self.Box`)) false false)
  (if condition
    (`self.RotateLeft`)
    (else
      (`self.RotateRight`))))

(fn `HanldeObjectPushing`
  (params (collisionBox :type "PrimitiveComponent Object Reference") (hand :type "SceneComponent Object Reference"))
  (bind _returnvalue (`SceneComponent.K2_GetComponentLocation` hand))
  (bind _box (`self.Box`))
  ;[1 1 1] For a more detailed comment, refer to the function HandleObjectPulling. The same thing is being done here, except for we're increasing the distance between the object and the controller.
  (`SceneComponent.K2_SetWorldLocation` _box (+ (* (`SceneComponent.GetForwardVector` hand) (+ (`KismetMathLibrary.Vector_Distance` (`SceneComponent.K2_GetComponentLocation` (`self.Box`)) _returnvalue) 2.0)) _returnvalue) true false)
  (`SceneComponent.K2_SetWorldLocation` collisionBox (`SceneComponent.K2_GetComponentLocation` _box) true false))

(fn `RotateLeft`
  (bind _box (`self.Box`))
  (`SceneComponent.K2_SetWorldRotation` _box (`KismetMathLibrary.MakeRotator` (.roll (`SceneComponent.K2_GetComponentRotation` _box)) (.pitch (`SceneComponent.K2_GetComponentRotation` _box)) (+ (.yaw (`SceneComponent.K2_GetComponentRotation` _box)) 2.0)) false false))

(fn `RotateRight`
  (bind _box (`self.Box`))
  (`SceneComponent.K2_SetWorldRotation` _box (`KismetMathLibrary.MakeRotator` (.roll (`SceneComponent.K2_GetComponentRotation` _box)) (.pitch (`SceneComponent.K2_GetComponentRotation` _box)) (+ (.yaw (`SceneComponent.K2_GetComponentRotation` _box)) -2.0)) false false))

(fn `UnfreezeObject`
  (bind _box (`self.Box`))
  ;[1 1 1] Re-enable physics, set the velocity that has been saved when the object was frozen, and enable gravity.
  (`PrimitiveComponent.SetSimulatePhysics` _box true)
  (`PrimitiveComponent.SetPhysicsLinearVelocity` _box (`self.savedVelocity`) false "None")
  (`PrimitiveComponent.SetEnableGravity` _box true)
  ;[1 1 1] Indicate that we are no longer frozen.
  (set `self.isFrozen` false))

(fn `UserConstructionScript`)