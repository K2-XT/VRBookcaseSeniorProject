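; BP_Create_New is a level-starter actor that, when its Grab function runs, creates a new saved level and opens EditorMap.
; It generates a name from the saved level count, caching it in a variable to avoid an off-by-one from double evaluation.
; SaveObjects gathers save-flagged BP_Interactive_Object actors' type, transform and frozen state, then writes them to the GameInstance's save slot.
; Grab then sets that name as the current level before loading the map.
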(fn `Fill Temp Interactables`
  (params (TempInteractables :type "Array of /Game/Blueprints/SavingLogic/InteractableSaveData Structure (by ref)"))
  (bind _outactors (`GameplayStatics.GetAllActorsOfClass` "/Game/Blueprints/InteractableObjects/BP_Interactive_Object.BP_Interactive_Object_C"))
  (for _array_element _outactors
    (if (`/Game/Blueprints/InteractableObjects/BP_Interactive_Object.doWeSaveObject` _array_element)
      (`KismetArrayLibrary.Array_Add` TempInteractables (make `/Game/Blueprints/SavingLogic/InteractableSaveData` (`/Game/Blueprints/InteractableObjects/BP_Interactive_Object.InteractableID` _array_element) (`SceneComponent.K2_GetComponentToWorld` (`/Game/Blueprints/InteractableObjects/BP_Interactive_Object.Box` _array_element)) (`/Game/Blueprints/InteractableObjects/BP_Interactive_Object.isFrozen` _array_element)))))
  (return))

(fn `Grab`
  (params (parent :type "SceneComponent Object Reference"))
  (locals (GeneratedLevelName :type String))
  ;[1 1 1] THIS MUST BE PROMOTED TO VARIABLE, NOT DIRECTLY PLUGGED IN, OTHERWISE IT'S BEING GENERATED TWICE, MAKING AN OFF BY ONE PROBLEM AND WE'RE SETTING CURRENT LEVEL TO +1 WHAT WE SENT INTO SAVE OBJECTS
  (bind _output_get (set `local.GeneratedLevelName` (`KismetTextLibrary.Conv_TextToString` (`|FormatText` "Level{int}" (`KismetArrayLibrary.Array_Length` (`/Game/Blueprints/SavingLogic/GlobalSaveGame.Levels` (`/Game/Blueprints/SavingLogic/RootGameInstance.SaveGameData` (`self.CurrentGameInstance`))))))))
  ;[1 1 1] Set the currently worked level to the generated level name and open the EditorMap.
  (`self.SaveObjects` _output_get)
  (set `/Game/Blueprints/SavingLogic/RootGameInstance.CurrentLevel` _output_get (`self.CurrentGameInstance`))
  (`GameplayStatics.OpenLevelBySoftObjectPtr` "/Game/Maps/EditorMap.EditorMap"))

(fn `SaveObjects`
  (params (CurrentLevelName :type String))
  (locals (TempInteractables :type "Array of /Game/Blueprints/SavingLogic/InteractableSaveData Structure"))
  (bind _currentgameinstance (`self.CurrentGameInstance`))
  (bind _savegamedata (`/Game/Blueprints/SavingLogic/RootGameInstance.SaveGameData` _currentgameinstance))
  (`self.Fill Temp Interactables` (`local.TempInteractables`))
  (`/Game/Blueprints/SavingLogic/GlobalSaveGame.SaveLevelData` (`/Game/Blueprints/SavingLogic/RootGameInstance.SaveGameData` (`self.CurrentGameInstance`)) CurrentLevelName (`local.TempInteractables`))
  (`GameplayStatics.SaveGameToSlot` _savegamedata (`/Game/Blueprints/SavingLogic/RootGameInstance.SaveSlotName` _currentgameinstance))
  (bind _interactablesdata (`/Game/Blueprints/SavingLogic/GlobalSaveGame.GetLevelData` _savegamedata (`local.CurrentLevelName`)))
  (`KismetSystemLibrary.PrintString` (`KismetTextLibrary.Conv_TextToString` (`|FormatText` "Was able to save {int} interactables into level: {string}" (`KismetStringLibrary.Conv_IntToString` (`KismetArrayLibrary.Array_Length` _interactablesdata)) (`local.CurrentLevelName`))) true true (struct :`R` 0.321725 :`G` 1.0 :`A` 1.0) 5.0))

(fn `UserConstructionScript`
  (`parent.UserConstructionScript`))