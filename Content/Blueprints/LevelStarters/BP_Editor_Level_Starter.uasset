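; BP_Editor_Level_Starter is a grabbable object that represents one level and opens it for work in the editor map.
; SetLevelHeld stores the level name and shows it on the text render.
; Grab runs the parent grab, writes the held name into the game instance's CurrentLevel, then opens the editor map.
; The event graph holds only disabled default events.
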(fn `Grab`
  (params (parent :type "SceneComponent Object Reference"))
  (`parent.Grab` null)
  ;[1 1 1] Set the currently worked-on level to the level held by this object and open up the editor map.
  (set `/Game/Blueprints/SavingLogic/RootGameInstance.currentLevel` (`self.heldLevelName`) (`self.currentGameInstance`))
  (`GameplayStatics.OpenLevelBySoftObjectPtr` "/Game/Maps/EditorMap.EditorMap"))

(fn `SetLevelHeld`
  (params (levelName :type String))
  (bind _output_get (set `self.heldLevelName` levelName))
  (`TextRenderComponent.K2_SetText` (`self.TextRender`) (`KismetTextLibrary.Conv_StringToText` _output_get)))

(fn `UserConstructionScript`
  (`parent.UserConstructionScript`))